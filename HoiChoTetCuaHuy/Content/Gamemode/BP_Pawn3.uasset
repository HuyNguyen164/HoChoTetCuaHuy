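; BP_Pawn3 is a player-controlled pawn with basic move and look controls through Enhanced Input.
; On BeginPlay it adds the IMC_Base mapping context to its player controller's input subsystem.
; IA_Move shifts the actor in local X and Y by a fixed multiple of the input, without delta-time scaling.
; IA_LookAround feeds its axes into controller yaw and pitch.
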(event `self.ReceiveBeginPlay`
  (bind _asplayer_controller (cast `PlayerController` (`self.GetController`)))
  (`EnhancedInputSubsystemInterface.AddMappingContext` (pcsubsystem `EnhancedInputLocalPlayerSubsystem` _asplayer_controller) "/Game/Input/IMC_Base.IMC_Base" 0 (struct)))

(event `EnhancedInput|/Game/Input/IA_Move`
  (params (ActionValue :type "Vector2D Structure") (ElapsedSeconds :type "Float (double-precision)") (TriggeredSeconds :type "Float (double-precision)") (InputAction :type "InputAction Object Reference" :default "/Game/Input/IA_Move.IA_Move"))
  (:`Triggered`
    (`self.K2_AddActorLocalOffset` (`KismetMathLibrary.MakeVector` (* ActionValue_X 5.0) (* ActionValue_Y 5.0)))))

(event `EnhancedInput|/Game/Input/IA_LookAround`
  (params (ActionValue :type "Vector2D Structure") (ElapsedSeconds :type "Float (double-precision)") (TriggeredSeconds :type "Float (double-precision)") (InputAction :type "InputAction Object Reference" :default "/Game/Input/IA_LookAround.IA_LookAround"))
  (:`Triggered`
    (`self.AddControllerYawInput` ActionValue_X)
    (`self.AddControllerPitchInput` ActionValue_Y)))

(fn `UserConstructionScript`)