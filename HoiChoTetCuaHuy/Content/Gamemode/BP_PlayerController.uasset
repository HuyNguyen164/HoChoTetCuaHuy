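; Player controller that cycles control between pawns when the IA_Possess input starts, noted as the P key.
; PossessNextPawn advances CurrentIndex, wraps it by the length of PossessablePawns and possesses that entry.
; A disconnected chain would fill the array from actors tagged Possessable, but it never runs, so no graph here populates the list.
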(event `EnhancedInput|/Game/Input/IA_Possess`
  (params (ActionValue :type Boolean) (ElapsedSeconds :type "Float (double-precision)") (TriggeredSeconds :type "Float (double-precision)") (InputAction :type "InputAction Object Reference" :default "/Game/Input/IA_Possess.IA_Possess"))
  ; Nhấn P để đổi pawn
  (:`Started`
    (`self.PossessNextPawn`)))

(fn `PossessNextPawn`
  (bind _output_get (set `self.CurrentIndex` (mod (+ (`self.CurrentIndex`) 1) (`KismetArrayLibrary.Array_Length` (`self.PossessablePawns`)))))
  (`self.Possess` (`|GetArrayItem` (`self.PossessablePawns`) _output_get)))

(fn `UserConstructionScript`)